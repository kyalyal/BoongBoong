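; Test Blueprint for cart race flow: start freeze, death feedback and respawn, with BeginPlay starting the SW_BP_CartGameMode timer.
; IfStart clears IsMove until a five-second timer restores it; IfDead loops back into it after a sound and immediately removed death UI.
; Respawn binds SportsCar_Pawn's OnDestroyed to a delayed spawn, possess and rebind, but nothing here initially calls it.
; CartDead and Resurrection are empty stubs; speed printing is a disconnected placeholder.
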(event Custom|IfStart
  ;[1 1 1] 시작할 때 5초 멈춰!
  (Variables|Default|SetIsMove false)
  (Development|PrintString (Utilities|String|ToString(Boolean) (Variables|Default|GetIsMove)))
  (Utilities|Time|SetTimerbyFunctionName 0 "WaitSecondForMove" 5.0))

(event Custom|IfDead
  ;[1 1 1] 죽었을 때
  (bind _returnvalue (UserInterface|CreateWidget "/Game/SW/Blueprint/DeadUi.DeadUi_C"))
  (UserInterface|Viewport|AddtoViewport _returnvalue 0)
  (Audio|PlaySound2D "/Game/StarterContent/Audio/Fire_Sparks01.Fire_Sparks01" 1.0 1.0 0.0 0 0)
  (Utilities|Time|SetTimerbyFunctionName 0 "CartDead" 5.0)
  (Widget|RemovefromParent _returnvalue)
  (Development|PrintString "UI 제거")
  ;[1 1 1] 시작할 때 5초 멈춰!
  (Variables|Default|SetIsMove false)
  (Development|PrintString (Utilities|String|ToString(Boolean) (Variables|Default|GetIsMove)))
  (Utilities|Time|SetTimerbyFunctionName 0 "WaitSecondForMove" 5.0))

(event Custom|PrintSpeed
  (Development|PrintString (Utilities|String|ToString(Float) (* (Math|Float|Absolute(Float) 0.0) 0.036))))

(event Custom|OnDestroyed_이벤트
  (params (DestroyedActor :type Actor%20Object%20Reference))
  ;[1 1 1] 리스폰 부분(pawn부분 건들려야해서 내일 물어보고 수정
  (Utilities|FlowControl|Delay 2.0)
  (bind _returnvalue (Game|SpawnActorfromClass "/Game/VehicleTemplate/Blueprints/SportsCar/SportsCar_Pawn.SportsCar_Pawn_C" (Variables|Default|GetSpawn%20Transform_0) "Undefined" "MultiplyWithRoot" 0 0))
  (Pawn|Possess (Variables|/Script/Engine.Pawn|GetLastHitBy (Game|Player|GetPlayerPawn 0)) _returnvalue)
  (CallFunction|Respawn))

(event Custom|Respawn
  ;[1 1 1] 리스폰 부분(pawn부분 건들려야해서 내일 물어보고 수정
  (bind _assports_car_pawn (Utilities|Casting|CastToSportsCar_Pawn (Game|Player|GetPlayerPawn 0)))
  (Game|AssignOnDestroyed _assports_car_pawn (delegate Custom|OnDestroyed_이벤트)))

(event EventBeginPlay
  ;[1 1 1] 연습용 시작후 상기 시작화면이동 후 타이머 로그 찍기 실행
  (bind _assw_bp_cart_game_mode (Utilities|Casting|CastToSW_BP_CartGameMode (Game|GetGameMode)))
  (Utilities|FlowControl|Sequence
    (:then_1
      (Class|BoongGameModeBase|StartTimer _assw_bp_cart_game_mode))))

(event Collision|EventActorBeginOverlap
  (params (OtherActor :type Actor%20Object%20Reference)))

(event EventTick
  (params (DeltaSeconds :type Float%20%28single-precision%29)))

(event Input|ActionEvents|InputActionDebuging
  (params (Key :type Key%20Structure :default "None"))
  ;[1 1 1] 연습용 시작후 상기 시작화면이동 후 타이머 로그 찍기 실행
)

(fn ConstructionScript)

(fn WaitSecondforMove
  (Variables|Default|SetIsMove true)
  (Development|PrintString (Utilities|String|ToString(Boolean) (Variables|Default|GetIsMove))))

(fn Resurrection
  ;[1 1 1] 부활 했을 때 발생되는 것
)

(fn CartDead)