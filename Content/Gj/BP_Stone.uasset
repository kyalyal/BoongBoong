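; BP_Stone is a construction-time placement tool that lines copies of a chosen mesh (MainMesh) along a spline.
; The construction script derives spacing from the mesh's X bounds plus an extra gap, then divides the spline length by it to get the count.
; It adds instanced static mesh instances at those distances in local space, setting location only; a tangent-rotation calculation is left unused.
; The event graph has no gameplay logic.
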(event EventBeginPlay)

(event Collision|EventActorBeginOverlap
  (params (OtherActor :type Actor%20Object%20Reference)))

(event EventTick
  (params (DeltaSeconds :type Float%20%28single-precision%29)))

(fn ConstructionScript
  (bind _main_mesh (Variables|Default|GetMain_Mesh))
  (bind _returnvalue (StaticMesh|GetBoundingBox _main_mesh))
  (Components|StaticMesh|SetStaticMesh (Variables|Default|GetInstancedStaticMesh) (Variables|Default|GetMain_Mesh))
  (bind _output_get (Variables|Default|Set간격길이 (+ (.x (- (.max _returnvalue) (.min _returnvalue))) (Variables|Default|Get여유길이))))
  (bind _output_get_2 (Variables|Default|Set몇개를설치하나? (Math|Float|Floor (/ (Spline|GetSplineLength (Variables|Default|GetSpline)) _output_get))))
  (for _index (range 0 _output_get_2)
    (Components|InstancedStaticMesh|AddInstance (Variables|Default|GetInstancedStaticMesh) (Math|Transform|MakeTransform (Spline|GetLocationatDistanceAlongSpline (Variables|Default|GetSpline) (* _index (Variables|Default|Get간격길이)) "Local") "0, 0, 0" "1.000000,1.000000,1.000000") false)))